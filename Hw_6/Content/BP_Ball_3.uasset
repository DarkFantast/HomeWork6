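; BP_Ball_3 is a ball actor that moves in a straight line and bounces off whatever blocks it.
; Tick moves it by a swept world offset along Direction at Speed, with no physics forces, and reflects Direction about the hit normal.
; Each bounce subtracts BaseSpeed, cut to a tenth of its initial value at BeginPlay, from Speed while Speed is above EndSpeed.
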(event `self.ReceiveTick`
  (params (DeltaSeconds :type "Float (single-precision)"))
  (bind _sweephitresult (`self.K2_AddActorWorldOffset` (* (* (`self.Direction`) (`self.Speed`)) DeltaSeconds) true))
  (bind (_bblockinghit _binitialoverlap _time _distance _location _impactpoint _normal) (`GameplayStatics.BreakHitResult` _sweephitresult))
  (if _bblockinghit
    (set `self.Direction` (`KismetMathLibrary.GetReflectionVector` (`self.Direction`) _normal))
    (if (not (<= (`self.Speed`) (`self.End Speed`)))
      (set `self.Speed` (- (`self.Speed`) (`self.BaseSpeed`))))))

(event `self.ReceiveBeginPlay`
  (set `self.BaseSpeed` (* (/ (`self.BaseSpeed`) 10.0) 1.0)))

(fn `UserConstructionScript`)